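; Main menu Game Mode that tracks players in the session lobby and starts the move to gameplay.
; On login it sends a Steam subsystem validation message to the Game Instance, stores the controller and initializes it; on logout it removes it and calls the update-all event.
; Travel notifies every stored controller through interface messages, waits briefly, then calls TravelToSelectedMap.
; Both that function and the update-all event have empty bodies here.
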(event `self.K2_PostLogin`
  (params (NewPlayer :type "PlayerController Object Reference"))
  ;[0.01562 0.01562 0.01562] OnPostLogin gets called when a player connects to the session for the first time.
  ;
  ; 1.We add this player to our Array of PlayerControllers so that we can later send updates to this individual
  ;
  ; 2. We initialize this player's PlayerController
  (`/Engine/EditorBlueprintResources/StandardMacros.IsValid` NewPlayer
    (:`Is Valid`
      (message `/Game/EscapeTheSeaons/Blueprints/Interfaces/BPI_GameInstance.BPI_ValidateSteamSubsystem` (`GameplayStatics.GetGameInstance`) NewPlayer)
      (`KismetArrayLibrary.Array_AddUnique` (`self.PlayerControllers`) NewPlayer)
      (message `/Game/EscapeTheSeaons/Blueprints/Interfaces/BPI_PlayerController.BPI_OC_Initialize` NewPlayer))))

(event `self.K2_OnLogout`
  (params (ExitingController :type "Controller Object Reference"))
  ;[0.01562 0.01562 0.01562] Removes the disconnected individual from the array of PlayerControllers and updates All Connected players that this individual disconnected
  (bind _playercontroller (message `/Game/EscapeTheSeaons/Blueprints/Interfaces/BPI_PlayerController.BPI_Get_PlayerController` ExitingController))
  (`/Engine/EditorBlueprintResources/StandardMacros.IsValid` _playercontroller
    (:`Is Valid`
      (`KismetArrayLibrary.Array_RemoveItem` (`self.PlayerControllers`) _playercontroller)
      (`self.BPI_MainMenu_UpdateAllConnectedPlayers`))))

(event `/Game/EscapeTheSeaons/Blueprints/Interfaces/BPI_GameMode.BPI_MainMenu_UpdateAllConnectedPlayers`
  ;[0.01562 0.01562 0.01562] Gets called when a player submits an update to the server
  ;
  ; Update examples:
  ;
  ; Player Connected, Changed ready status, Changed Skin, Host changed Match Settings, Player Disconnected
)

(event `/Game/EscapeTheSeaons/Blueprints/Interfaces/BPI_GameMode.BPI_TravelTo_GamePlay`
  ;[0.01562 0.01562 0.01562] Travels to Gameplay Map - Called when Host decided to start the game
  (for _array_element (`self.PlayerControllers`)
    (message `/Game/EscapeTheSeaons/Blueprints/Interfaces/BPI_PlayerController.BPI_OC_HandleServerTravel` _array_element))
  (`KismetSystemLibrary.Delay` 1.0)
  (`self.TravelTo_SelectedMap`))

(fn `TravelTo_SelectedMap`)

(fn `UserConstructionScript`)