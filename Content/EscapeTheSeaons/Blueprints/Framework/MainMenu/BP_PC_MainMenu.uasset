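; Main menu lobby PlayerController that sets up each client's menu and syncs its player info with the server.
; On initialization it creates the main menu widget, then submits the GameInstance profile, flagged with host status, to the server.
; The server stores it, tells the GameMode to update all connected players, and has the owning client save a copy for gameplay.
; The server-travel transition event is an empty stub.
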(event `/Game/EscapeTheSeaons/Blueprints/Interfaces/BPI_PlayerController.BPI_OC_Initialize`
  ;[0.01562 0.01562 0.01562] 1. Initializes the client: Handles Map transition fades > Creates lobby UI > Submits PlayerInfo to Server
  (`self.OC_Initialize`))

(event `OC_Initialize`
  ;[0.01562 0.01562 0.01562] 1. Initializes the client: Handles Map transition fades > Creates lobby UI > Submits PlayerInfo to Server
  (`self.InitializePlayerController`))

(event `SVR_SubmitUpdate`
  (params (Player_Info :type "/Game/EscapeTheSeaons/Data/Structs/ST_ConnectedPlayer Structure"))
  ;[0.01562 0.01562 0.01562] Updates the server when this players PlayerInfo has changed (Skin, Ready status). Also saves a local copy of the PlayerInfo structure in the players GameInstance
  (set `self.PlayerInfo` Player_Info)
  (message `/Game/EscapeTheSeaons/Blueprints/Interfaces/BPI_GameMode.BPI_MainMenu_UpdateAllConnectedPlayers` (`GameplayStatics.GetGameMode`))
  (`self.OC_SaveInformation` (`self.PlayerInfo`)))

(event `OC_SaveInformation`
  (params (PlayerInfo :type "/Game/EscapeTheSeaons/Data/Structs/ST_ConnectedPlayer Structure"))
  ;[0.01562 0.01562 0.01562] Saves a copy of player info on the owning clients GameInstance. So we can acces it in the Gameplay_GameMode
  (message `/Game/EscapeTheSeaons/Blueprints/Interfaces/BPI_GameInstance.BPI_Save_PlayerProfileOnGameInstance` (`GameplayStatics.GetGameInstance`) PlayerInfo))

(event `/Game/EscapeTheSeaons/Blueprints/Interfaces/BPI_PlayerController.BPI_OC_HandleServerTravel`
  ;[0.01562 0.01562 0.01562] Called when Server travels to Gameplay Map: Creates transition screens
  (`self.OC_Create_MapTravel_Transition`))

(event `OC_Create_MapTravel_Transition`
  ;[0.01562 0.01562 0.01562] Called when Server travels to Gameplay Map: Creates transition screens
)

(event `Key|One`
  (params (Key :type "Key Structure")))

(fn `BPI_Get_PlayerController`
  (returns (PlayerController :type "PlayerController Object Reference"))
  (return null))

(fn `Create_MainMenu_WBP`
  (bind _wbp_mainmenu (`self.WBP_MainMenu`)
    (:`then`
      (if (not (`Widget.IsInViewport` _wbp_mainmenu))
        (`UserWidget.AddToViewport` _wbp_mainmenu 0 :!label _label)))
    (:`else`
      (bind _returnvalue (`|CreateWidget` "/Game/EscapeTheSeaons/Widgets/MainMenu/WBP_MainMenu.WBP_MainMenu_C" (`GameplayStatics.GetPlayerController` 0)))
      (set `self.WBP_MainMenu` _returnvalue)
      (goto _label))))

(fn `Fetch Player Info from Game Instance`
  (returns (PlayerInfo :type "/Game/EscapeTheSeaons/Data/Structs/ST_ConnectedPlayer Structure (by ref)"))
  (bind _structout (setmembers `/Game/EscapeTheSeaons/Data/Structs/ST_ConnectedPlayer` :`StructRef` (`self.PlayerInfo`) :`bIsHost?` (`KismetSystemLibrary.IsServer`) :`PlayerInfo` (`/Game/EscapeTheSeaons/Blueprints/FunctionLibary/BFL_EscapeTheSeasons.BFL_Get_PlayerInfo`)))
  (return _structout))

(fn `InitializePlayerController`
  (`self.Create_MainMenu_WBP`)
  (bind _playerinfo (`self.Fetch Player Info from Game Instance`))
  (`self.SVR_SubmitUpdate` _playerinfo))

(fn `UserConstructionScript`)