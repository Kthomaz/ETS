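; Game instance for Escape The Seasons that holds the save object, a copy of player info and online session handling.
; On Init it creates a save object, replaces it with the saved slot if one exists, then calls a still-empty audio setup.
; Interface events create two-connection sessions, destroy them and check Steam login through a delayed, counted macro; joining is a stub.
; Network and travel errors destroy the local player's session.
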(event `self.ReceiveInit`
  ;[0.01562 0.01562 0.01562] Initialize
  (`self.Create_SaveGameObject`))

(event `Create_SaveGameObject`
  ;[0.01562 0.01562 0.01562] Initialize
  (bind _returnvalue (`GameplayStatics.CreateSaveGameObject` "/Game/EscapeTheSeaons/Blueprints/SaveGames/BP_SG_EscapeTheSeasons.BP_SG_EscapeTheSeasons_C"))
  (set `self.BP_SG_EscapeTheSeasons` _returnvalue)
  (bind _returnvalue_2 (`GameplayStatics.DoesSaveGameExist` "General_SaveSlot"))
  (if _returnvalue_2
    (`self.Load_BP_SG_EscapeTheSeasons`)))

(event `Load_BP_SG_EscapeTheSeasons`
  ;[0.01562 0.01562 0.01562] Initialize
  (bind _returnvalue (`GameplayStatics.LoadGameFromSlot` "General_SaveSlot"))
  (bind _asbp_sg_escape_the_seasons (cast `/Game/EscapeTheSeaons/Blueprints/SaveGames/BP_SG_EscapeTheSeasons` _returnvalue))
  (set `self.BP_SG_EscapeTheSeasons` _asbp_sg_escape_the_seasons)
  (`self.Initialize_AudioSettings`))

(event `/Game/EscapeTheSeaons/Blueprints/Interfaces/BPI_GameInstance.BPI_Save_PlayerProfileOnGameInstance`
  (params (PlayerInfo :type "/Game/EscapeTheSeaons/Data/Structs/ST_ConnectedPlayer Structure"))
  ;[0.01562 0.01562 0.01562] Saves a copy of player info on the owning clients GameInstance. So we can acces it in the Gameplay_GameMode
  (set `self.Player Info` PlayerInfo))

(event `/Game/EscapeTheSeaons/Blueprints/Interfaces/BPI_GameInstance.BPI_ValidateSteamSubsystem`
  (params (PlayerController :type "PlayerController Object Reference"))
  ;[0.01562 0.01562 0.01562] ValidatedSteamSubsystem after a valid controller check in the playercontroller
  (`self.ValidateSteamSubsystem` PlayerController))

(event `Initialize_AudioSettings`)

(event `/Game/EscapeTheSeaons/Blueprints/Interfaces/BPI_GameInstance.BPI_JoinSession`
  (params (SessionToJoin :type "BlueprintSessionResult Structure")))

(event `/Game/EscapeTheSeaons/Blueprints/Interfaces/BPI_GameInstance.BPI_CreateSession`
  ;[0.01562 0.01562 0.01562] Creates a session with session settings
  (`CreateSessionCallbackProxyAdvanced.CreateAdvancedSession` :`PlayerController` (`GameplayStatics.GetPlayerController` 0) :`PublicConnections` 2
    (:`OnSuccess`
      (`KismetSystemLibrary.PrintString` "BP_GI_BPI_CreateSession_SessionCreated" true true (struct :`G` 1.0 :`A` 1.0) 100.0))))

(event `/Game/EscapeTheSeaons/Blueprints/Interfaces/BPI_GameInstance.BPI_DestroySessionCaller`
  (params (PlayerController :type "PlayerController Object Reference"))
  ;[0.01562 0.01562 0.01562] Destroys the Session of the caller
  (`DestroySessionCallbackProxy.DestroySession` PlayerController
    (:`OnSuccess`
      (`KismetSystemLibrary.PrintString` "BP_GI_BPI_DestroySessionCaller : SessionDestroyed" true true (struct :`R` 1.0 :`A` 1.0) 100.0))))

(event `self.HandleNetworkError`
  (params (FailureType :type "ENetworkFailure Enum" :default "NetDriverAlreadyExists") (bIsServer :type Boolean))
  ;[0.01562 0.01562 0.01562] Handle displaying Network and Travel Errors
  (`self.BPI_DestroySessionCaller` (`GameplayStatics.GetPlayerController` 0)))

(event `self.HandleTravelError`
  (params (FailureType :type "ETravelFailure Enum" :default "NoLevel"))
  ;[0.01562 0.01562 0.01562] Handle displaying Network and Travel Errors
  (`self.BPI_DestroySessionCaller` (`GameplayStatics.GetPlayerController` 0)))

(fn `BPI_Get_SaveGameObject`
  (returns (SaveGame :type "/Game/EscapeTheSeaons/Blueprints/SaveGames/BP_SG_EscapeTheSeasons Object Reference"))
  (return (`self.BP_SG_EscapeTheSeasons`)))